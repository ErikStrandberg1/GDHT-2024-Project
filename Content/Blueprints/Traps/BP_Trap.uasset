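; BP_Trap is a single-use trap that flings a vehicle that touches it.
; Its Collision overlap passes a DoOnce that is never reset, so the first overlap spends it, even from a non-vehicle or an immune car.
; A non-immune VehicleAdvPawn goes to Fling, which applies a velocity-change impulse to its mesh using RandomValue outputs, with all three axes negated on a coin flip.
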(event `self.Collision.OnComponentBeginOverlap`
  (params (OverlappedComponent :type "PrimitiveComponent Object Reference") (OtherActor :type "Actor Object Reference") (OtherComp :type "PrimitiveComponent Object Reference") (OtherBodyIndex :type Integer) (bFromSweep :type Boolean) (SweepResult :type "HitResult Structure (by ref)"))
  (`/Engine/EditorBlueprintResources/StandardMacros.DoOnce` false
    (:`Completed`
      (if (!= OtherActor self)
        (bind _asvehicle_adv_pawn (cast `/Game/Blueprints/Vehicles/Default/VehicleAdvPawn` OtherActor))
        (if (not (`/Game/Blueprints/Vehicles/Default/VehicleAdvPawn.Immune?` _asvehicle_adv_pawn))
          (`self.Fling` _asvehicle_adv_pawn))))))

(fn `Fling`
  (params (WhichCar :type "/Game/Blueprints/Vehicles/Default/VehicleAdvPawn Object Reference"))
  (bind (_x _y _returnvalue3) (`self.RandomValue`))
  (bind _mesh (`WheeledVehiclePawn.Mesh` WhichCar))
  (if (`KismetMathLibrary.RandomBool`)
    (`PrimitiveComponent.AddImpulse` _mesh (`KismetMathLibrary.MakeVector` _x _y _returnvalue3) "None" true)
    (else
      (`PrimitiveComponent.AddImpulse` _mesh (`KismetMathLibrary.MakeVector` (* _x -1.0) (* _y -1.0) (* _returnvalue3 -1.0)) "None" true))))

(fn `UserConstructionScript`)